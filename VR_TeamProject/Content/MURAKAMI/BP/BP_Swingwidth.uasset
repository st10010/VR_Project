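; BP_Swingwidth is an actor intended to detect sword swings, judging by its comments and debug message.
; On BeginPlay it loops over actors of a class, and each Tick it snaps to the loop's current element without sweep.
; A check compares its own velocity magnitude to a threshold and prints that the sword was swung.
; That check sits on the false side of a constant-true branch, so it never runs as written.
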(event `self.ReceiveTick`
  (params (DeltaSeconds :type "Float (single-precision)"))
  ;[1 1 1] 剣に向かって移動する
  (`self.K2_SetActorLocation` (`self.K2_GetActorLocation` (stale `self.ReceiveBeginPlay` _array_element))) ; ターゲットのの座標に指定
  (if true
    _
    (elif (> (`KismetMathLibrary.VSize` (`self.GetVelocity` self)) 800.0)
      (`KismetSystemLibrary.PrintString` "剣がふられた"))))

(event `self.ReceiveBeginPlay`
  ;[1 1 1] 剣に向かって移動する
  (`GameplayStatics.GetAllActorsOfClass` null) ; レベル内の特定のアクタを参照
  (for _array_element _
    _))

(fn `UserConstructionScript`)