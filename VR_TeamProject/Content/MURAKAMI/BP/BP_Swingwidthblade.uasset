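; Sword-swing detection actor that follows a BP_Target actor and reports when the sword is swung.
; BeginPlay runs an empty loop over all BP_Target actors, and Tick snaps this actor to the location of that loop's leftover element without sweep.
; Each Tick then compares the magnitude of the actor's own velocity to a fixed threshold and prints a debug message when it is exceeded.
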(event `self.ReceiveTick`
  (params (DeltaSeconds :type "Float (single-precision)"))
  ;[1 1 1] 剣に向かって移動する
  (`self.K2_SetActorLocation` (`self.K2_GetActorLocation` (stale `self.ReceiveBeginPlay` _array_element))) ; ターゲットのの座標に指定
  (if (> (`KismetMathLibrary.VSize` (`self.GetVelocity` self)) 1000.0)
    (`KismetSystemLibrary.PrintString` "剣がふられた")))

(event `self.ReceiveBeginPlay`
  ;[1 1 1] 剣に向かって移動する
  (bind _outactors (`GameplayStatics.GetAllActorsOfClass` "/Game/MURAKAMI/BP/BP_Target.BP_Target_C")) ; レベル内の特定のアクタを参照
  (for _array_element _outactors
    _))

(fn `UserConstructionScript`)